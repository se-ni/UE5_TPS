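; BP_MainCharacter is the main character Blueprint, with a hold-to-zoom camera on the left mouse button.
; BeginPlay caches the camera's relative transform and the spring arm length.
; Pressing the button collapses the arm to zero and resets the camera's relative transform, pulling the view in to the arm's pivot.
; Releasing it restores both cached values instantly, without interpolation.
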(event `self.ReceiveBeginPlay`
  (set `self.위치` (`SceneComponent.GetRelativeTransform` (`self.Camera`)))
  (set `self.타깃 암 길이` (`SpringArmComponent.TargetArmLength` (`self.SpringArm`))))

(event `Key|LeftMouseButton`
  (params (Key :type "Key Structure"))
  (bind _camera (`self.Camera`))
  (bind _springarm (`self.SpringArm`))
  (:`Pressed`
    (set `SpringArmComponent.TargetArmLength` 0.0 _springarm)
    (`SceneComponent.K2_SetRelativeTransform` _camera (`KismetMathLibrary.MakeTransform` (-3.137607 -27.0 -35.863009)) false false))
  (:`Released`
    (set `SpringArmComponent.TargetArmLength` (`self.타깃 암 길이`) _springarm)
    (`SceneComponent.K2_SetRelativeTransform` _camera (`self.위치`) false false)))

(fn `UserConstructionScript`)